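; Test actor that uses a physics constraint's linear drive to move StaticMesh and Cube until they overlap.
; While Open has its gate open, Tick breaks and rebuilds the constraint each frame, reapplying drive parameters and a target from the constraint-to-mesh offset scaled by Power.
; StaticMesh overlapping Cube disables the drive, zeroes the target and closes the gate, with debug prints reporting clicks and overlap results.
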(event OnComponentBeginOverlap(StaticMesh)
  (params (OverlappedComponent :type Primitive%20Component%20Object%20Reference) (OtherActor :type Actor%20Object%20Reference) (OtherComp :type Primitive%20Component%20Object%20Reference) (OtherBodyIndex :type Integer) (bFromSweep :type Boolean) (SweepResult :type Hit%20Result%20Structure%20%28by%20ref%29))
  (bind _physicsconstraint (Variables|Default|GetPhysicsConstraint))
  (if (== OtherComp (Variables|Default|GetCube))
    (Development|PrintString "True")
    (Class|PhysicsConstraintComponent|SetLinearPositionDrive _physicsconstraint false false false)
    (Class|PhysicsConstraintComponent|SetLinearPositionTarget _physicsconstraint (Math|Vector|MakeVector 0.0 0.0 0.0))
    (CallFunction|Close)
    (else
      (Development|PrintString "False"))))

(event Custom|Open
  (bind _physicsconstraint (Variables|Default|GetPhysicsConstraint))
  (bind _param (Variables|Default|GetParam))
  (Class|PhysicsConstraintComponent|SetLinearPositionDrive (Variables|Default|GetPhysicsConstraint) true true true)
  (Development|PrintString "Click")
  (Utilities|FlowControl|Gate true) ; enters at Open
)

(event Custom|Close
  (bind _physicsconstraint (Variables|Default|GetPhysicsConstraint))
  (bind _param (Variables|Default|GetParam))
  (Utilities|FlowControl|Gate true) ; enters at Close
)

(event EventBeginPlay
  (Class|PhysicsConstraintComponent|SetLinearPositionDrive (Variables|Default|GetPhysicsConstraint) true true true))

(event EventTick
  (params (DeltaSeconds :type Float%20%28single-precision%29))
  (bind _physicsconstraint (Variables|Default|GetPhysicsConstraint))
  (bind _param (Variables|Default|GetParam))
  (Utilities|FlowControl|Gate true
    (:Exit
      (Class|PhysicsConstraintComponent|BreakConstraint _physicsconstraint)
      (Class|PhysicsConstraintComponent|SetLinearDriveParams _physicsconstraint (.x _param) (.y _param) (.z _param))
      (Class|PhysicsConstraintComponent|SetLinearPositionTarget _physicsconstraint (* (- (Transformation|GetWorldLocation _physicsconstraint) (Transformation|GetWorldLocation (Variables|Default|GetStaticMesh))) (Variables|Default|GetPower)))
      (Class|PhysicsConstraintComponent|SetConstrainedComponents _physicsconstraint (Variables|Default|GetStaticMesh) "None" (Variables|Default|GetCube) "None"))))

(fn ConstructionScript)