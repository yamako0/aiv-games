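; BP_Bullet is a bullet actor that deals damage through a hitscan-style line trace.
; Every Tick, LineTrace casts a debug-drawn Visibility trace from the actor's location along the StaticMesh forward vector over a fixed range.
; It passes the hit actor straight to ApplyDamage with the Damage variable, so damage repeats each frame a target stays in line.
; The graphs contain no movement or destroy logic.
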(event EventTick
  (params (DeltaSeconds :type Float%20%28single-precision%29))
  (CallFunction|LineTrace))

(fn ConstructionScript)

(fn LineTrace
  (bind _returnvalue (Transformation|GetActorLocation))
  (bind _outhit (Collision|LineTraceByChannel _returnvalue (+ _returnvalue (* (Math|Vector|GetForwardVector (Variables|Default|GetStaticMesh)) 2e+03)) "TraceTypeQuery1" false 0 "ForOneFrame"))
  (Game|Damage|ApplyDamage (.HitActor (Collision|BreakHitResult _outhit)) (Variables|Default|GetDamage) 0 0)
  (return))