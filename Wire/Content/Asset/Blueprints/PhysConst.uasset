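; PhysConst is an actor Blueprint that drives a physics constraint with a linear velocity motor.
; BeginPlay enables velocity drive on all three axes and disables position drive.
; At BeginPlay and every Tick, it applies spring, damping and force limit from Param, then sets the velocity target to the constraint-to-mesh relative-location direction scaled by Power.
; It also sets a position target at the constraint's relative location, although that drive is off.
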(event EventBeginPlay
  (bind _physicsconstraint (Variables|Default|GetPhysicsConstraint))
  (bind _physicsconstraint_2 (Variables|Default|GetPhysicsConstraint))
  (bind _physicsconstraint_3 (Variables|Default|GetPhysicsConstraint))
  (bind _param (Variables|Default|GetParam))
  (Class|PhysicsConstraintComponent|SetLinearVelocityDrive _physicsconstraint true true true)
  (Class|PhysicsConstraintComponent|SetLinearPositionDrive _physicsconstraint false false false)
  (Utilities|FlowControl|Sequence
    (:then_0
      (Class|PhysicsConstraintComponent|SetLinearDriveParams _physicsconstraint_3 (.x _param) (.y _param) (.z _param))
      (Class|PhysicsConstraintComponent|SetLinearVelocityTarget _physicsconstraint_3 (* (Math|Vector|Normalize (- (Variables|/Script/Engine.SceneComponent|GetRelativeLocation (Variables|Default|GetStaticMesh)) (Variables|/Script/Engine.SceneComponent|GetRelativeLocation _physicsconstraint_3))) (Variables|Default|GetPower))))
    (:then_1
      (Class|PhysicsConstraintComponent|SetLinearPositionTarget _physicsconstraint_2 (Variables|/Script/Engine.SceneComponent|GetRelativeLocation _physicsconstraint_2)))))

(event EventTick
  (params (DeltaSeconds :type Float%20%28single-precision%29))
  (bind _physicsconstraint (Variables|Default|GetPhysicsConstraint))
  (bind _physicsconstraint_2 (Variables|Default|GetPhysicsConstraint))
  (bind _param (Variables|Default|GetParam))
  (Utilities|FlowControl|Sequence
    (:then_0
      (Class|PhysicsConstraintComponent|SetLinearDriveParams _physicsconstraint_2 (.x _param) (.y _param) (.z _param))
      (Class|PhysicsConstraintComponent|SetLinearVelocityTarget _physicsconstraint_2 (* (Math|Vector|Normalize (- (Variables|/Script/Engine.SceneComponent|GetRelativeLocation (Variables|Default|GetStaticMesh)) (Variables|/Script/Engine.SceneComponent|GetRelativeLocation _physicsconstraint_2))) (Variables|Default|GetPower))))
    (:then_1
      (Class|PhysicsConstraintComponent|SetLinearPositionTarget _physicsconstraint (Variables|/Script/Engine.SceneComponent|GetRelativeLocation _physicsconstraint)))))

(fn ConstructionScript)