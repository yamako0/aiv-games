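; Physics test actor that pulls a static mesh toward a physics constraint's location and joins it to a Cube component.
; While the gate is open, Tick adds velocity scaled by distance and Power, and re-sets the constrained components every frame.
; Open starts the pull; overlapping the Cube cancels the mesh's linear velocity and closes the gate.
; Debug prints remain, and the BreakConstraint call is not wired to any event.
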(event OnComponentBeginOverlap(StaticMesh)
  (params (OverlappedComponent :type Primitive%20Component%20Object%20Reference) (OtherActor :type Actor%20Object%20Reference) (OtherComp :type Primitive%20Component%20Object%20Reference) (OtherBodyIndex :type Integer) (bFromSweep :type Boolean) (SweepResult :type Hit%20Result%20Structure%20%28by%20ref%29))
  (bind _staticmesh (Variables|Default|GetStaticMesh))
  (if (== OtherComp (Variables|Default|GetCube))
    (Development|PrintString "True")
    (bind _returnvalue (Physics|GetPhysicsLinearVelocity _staticmesh "None"))
    (Physics|SetPhysicsLinearVelocity _staticmesh (* _returnvalue -1.0) true "None")
    (CallFunction|Close)
    (else
      (Development|PrintString "False"))))

(event Custom|Open
  (bind _staticmesh (Variables|Default|GetStaticMesh))
  (bind _physicsconstraint (Variables|Default|GetPhysicsConstraint))
  (Development|PrintString "Click")
  (Utilities|FlowControl|Gate true) ; enters at Open
)

(event Custom|Close
  (bind _staticmesh (Variables|Default|GetStaticMesh))
  (bind _physicsconstraint (Variables|Default|GetPhysicsConstraint))
  (Utilities|FlowControl|Gate true) ; enters at Close
)

(event EventTick
  (params (DeltaSeconds :type Float%20%28single-precision%29))
  (bind _staticmesh (Variables|Default|GetStaticMesh))
  (bind _physicsconstraint (Variables|Default|GetPhysicsConstraint))
  (Utilities|FlowControl|Gate true
    (:Exit
      (Physics|SetPhysicsLinearVelocity _staticmesh (* (- (Transformation|GetWorldLocation _physicsconstraint) (Transformation|GetWorldLocation _staticmesh)) (Variables|Default|GetPower)) true "None")
      (Class|PhysicsConstraintComponent|SetConstrainedComponents _physicsconstraint (Variables|Default|GetStaticMesh) "None" (Variables|Default|GetCube) "None"))))

(fn ConstructionScript)